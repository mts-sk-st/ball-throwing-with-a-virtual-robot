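; BP_Robot is a robot arm actor that other Blueprints position and pose, and that grabs balls it touches.
; Custom events set the actor's location and the relative rotations of the root, BaseToArm1 and Arm1ToArm2 joint components.
; On a hit with a BP_Ball, it turns off the ball's physics and attaches it to the hand_to_ball socket on the Hand.
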(event `SetRobotPosition`
  (params (Position :type "Vector Structure"))
  ;[1 1 1] Custom event to set robots position from other blueprints
  (`self.K2_SetActorLocation` Position))

(event `SetJointAngles`
  (params (Base :type "Rotator Structure") (Arm1 :type "Rotator Structure") (Arm2 :type "Rotator Structure"))
  ;[1 1 1] Custom event to set all of the changeable joint angles from other blueprints
  (`SceneComponent.K2_SetRelativeRotation` (`self.DefaultSceneRoot`) Base false false)
  (`SceneComponent.K2_SetRelativeRotation` (`self.base_to_arm1`) Arm1 false false)
  (`SceneComponent.K2_SetRelativeRotation` (`self.arm1_to_arm2`) Arm2 false false))

(event `self.ReceiveHit`
  (params (MyComp :type "PrimitiveComponent Object Reference") (Other :type "Actor Object Reference") (OtherComp :type "PrimitiveComponent Object Reference") (bSelfMoved :type Boolean) (HitLocation :type "Vector Structure") (HitNormal :type "Vector Structure") (NormalImpulse :type "Vector Structure") (Hit :type "HitResult Structure (by ref)"))
  ;[1 1 1] Add hit event for when collision is detected with a throwable object, that attaches it to the robot at the hands socket
  (bind _asbp_ball (cast `/Game/VirtualRealityBP/Blueprints/BP_Ball` Other))
  (`PrimitiveComponent.SetSimulatePhysics` (`StaticMeshActor.StaticMeshComponent` _asbp_ball) false)
  (`SceneComponent.K2_AttachToComponent` (`Actor.RootComponent` _asbp_ball) (`self.hand`) "hand_to_ball" "SnapToTarget" "KeepRelative" "KeepRelative" true))

(fn `UserConstructionScript`)