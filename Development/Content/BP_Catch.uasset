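; BP_Catch is the robot's reachable-space actor, which makes the robot catch thrown balls that overlap it.
; On overlap with a BP_Ball, it moves the whole robot to the ball's location, offset downward so the hand meets it.
; ManipulateRobot is an unused placeholder for future IK joint angles, returning zero rotations.
; Tick watches BallCount and reloads the current level after a delay once it reaches zero.
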(event `self.ReceiveActorBeginOverlap`
  (params (OtherActor :type "Actor Object Reference"))
  (bind _robot (`self.Robot`))
  ;[1 1 1] When thrown object overlaps robots reachable space, call manipulate robot to get new joint angles, then set those joint angles
  (bind _asbp_ball (cast `/Game/VirtualRealityBP/Blueprints/BP_Ball` OtherActor))
  (set `self.bGenerateOverlapEventsDuringLevelStreaming` false)
  (bind _robotposition (`self.SimpleManipulateRobot` _asbp_ball))
  (`/Engine/EditorBlueprintResources/StandardMacros.IsValid` _robot
    (:`Is Valid`
      (`/Game/Robot_Model/BP_Robot.SetRobotPosition` _robot _robotposition))))

(event `self.ReceiveTick`
  (params (DeltaSeconds :type "Float (single-precision)"))
  ;[1 1 1] When ball count reaches zero, reload the level
  (if (== (`self.BallCount`) 0)
    (`KismetSystemLibrary.Delay` 5.0)
    (bind _returnvalue (`GameplayStatics.GetCurrentLevelName` true))
    (`GameplayStatics.OpenLevel` (`KismetStringLibrary.Conv_StringToName` _returnvalue))))

(fn `ManipulateRobot`
  (params (Ball :type "/Game/VirtualRealityBP/Blueprints/BP_Ball Object Reference"))
  (returns (Base :type "Rotator Structure") (Arm1 :type "Rotator Structure") (Arm2 :type "Rotator Structure"))
  ;[1 1 1] Function to calculate joint angles when IK is implemented
  (return (`KismetMathLibrary.MakeRotator` 0.0) (`KismetMathLibrary.MakeRotator` 0.0) (`KismetMathLibrary.MakeRotator` 0.0)))

(fn `SimpleManipulateRobot`
  (params (Ball :type "/Game/VirtualRealityBP/Blueprints/BP_Ball Object Reference"))
  (returns (RobotPosition :type "Vector Structure"))
  ;[1 1 1] Simple robot manipulation to move the whole robot into a position where the hand hits the thrown ball
  (return (`KismetMathLibrary.MakeVector` (.x (`self.K2_GetActorLocation` Ball)) (.y (`self.K2_GetActorLocation` Ball)) (- (.z (`self.K2_GetActorLocation` Ball)) 292.0))))

(fn `UserConstructionScript`)